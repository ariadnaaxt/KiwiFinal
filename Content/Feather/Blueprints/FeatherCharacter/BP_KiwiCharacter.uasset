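; Kiwi character Blueprint that turns player input into click and dialog interaction events.
; The IA_Click input action broadcasts a click delegate.
; Pressing E runs a sphere trace around the character and broadcasts ExecuteDialog for the first hit actor tagged Interactable, passing that actor's second tag as the dialog identifier.
; A separate interaction event destroys the stored text handle actor if it is valid.
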(event `self.OnInteractionPressed`
  (bind _as_bp_text_handle (`self.As BP Text Handle`))
  (`/Engine/EditorBlueprintResources/StandardMacros.IsValid` _as_bp_text_handle
    (:`Is Valid`
      (`self.K2_DestroyActor` _as_bp_text_handle))))

(event `EnhancedInput|/Game/Feather/Blueprints/FeatherCharacter/Input/Actions/IA_Click`
  (params (ActionValue :type Boolean) (ElapsedSeconds :type "Float (double-precision)") (TriggeredSeconds :type "Float (double-precision)") (InputAction :type "InputAction Object Reference" :default "/Game/Feather/Blueprints/FeatherCharacter/Input/Actions/IA_Click.IA_Click"))
  (:`Triggered`
    (`self.ClickActionDelegate`)))

(event `Key|E`
  (params (Key :type "Key Structure"))
  (bind _returnvalue (`self.K2_GetActorLocation`))
  (:`Pressed`
    (bind _outhits (`KismetSystemLibrary.SphereTraceMulti` _returnvalue _returnvalue 110.0 "TraceTypeQuery1" false (`|MakeArray` self :!type "Actor Object Reference")))
    (for _array_element _outhits
      (bind (_bblockinghit _binitialoverlap _time _distance _location _impactpoint _normal _impactnormal _physmat _hitactor) (`GameplayStatics.BreakHitResult` _array_element))
      (if (`self.ActorHasTag` _hitactor "Interactable")
        (`self.ExecuteDialog` (`|GetArrayItem` (`Actor.Tags` _hitactor) 1))
        (break)))))

(fn `UserConstructionScript`)