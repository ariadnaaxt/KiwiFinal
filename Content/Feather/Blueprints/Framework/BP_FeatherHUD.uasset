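; BP_FeatherHUD is the HUD Blueprint that owns the player's main UI widget and exposes gameplay-facing calls for showing information.
; On BeginPlay it creates a WBP_UI widget, stores it as PlayerUI and adds it to the viewport.
; Its events and functions forward lore text, objective text, dialog and comic requests to that widget, with lore text cleared after a delay of the given duration.
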(event `self.ReceiveBeginPlay`
  (bind _returnvalue (`|CreateWidget` "/Game/Feather/Widgets/WBP_UI.WBP_UI_C"))
  (bind _output_get (set `self.PlayerUI` _returnvalue))
  (`UserWidget.AddToViewport` _output_get 0))

(event `ShowLoreText`
  (params (InText :type Text) (Duration :type "Float (single-precision)"))
  (`/Game/Feather/Widgets/WBP_UI.SetLoreText` (`self.PlayerUI`) InText)
  (`KismetSystemLibrary.Delay` Duration)
  (`/Game/Feather/Widgets/WBP_UI.ClearLoreText` (`self.PlayerUI`)))

(event `SetObjectiveText`
  (params (InText :type Text))
  (`/Game/Feather/Widgets/WBP_UI.SetObjectiveText` (`self.PlayerUI`) InText))

(fn `StartComic`
  (params (InComicImages :type "Array of Texture2D Object Reference (by ref)"))
  (bind _playerui (`self.PlayerUI`))
  (`/Engine/EditorBlueprintResources/StandardMacros.IsValid` _playerui
    (:`Is Valid`
      (`/Game/Feather/Widgets/WBP_UI.StartComic` _playerui InComicImages))))

(fn `StartDialog`
  (params (DialogConfig :type "Array of DialogConfig Structure (by ref)"))
  (bind _playerui (`self.PlayerUI`))
  (`/Engine/EditorBlueprintResources/StandardMacros.IsValid` _playerui
    (:`Is Valid`
      (`/Game/Feather/Widgets/WBP_UI.StartDialog` _playerui DialogConfig))))

(fn `UserConstructionScript`)