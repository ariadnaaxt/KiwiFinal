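; BP_TextHandle is a trigger actor that shows lore text on screen when the kiwi character enters its box.
; It caches the BP_FeatherHUD reference one tick after BeginPlay.
; On overlap with BP_KiwiCharacter, it passes its text and duration to the HUD's ShowLoreText.
; A DoOnce flag limits this to a single showing unless the actor is marked repeatable.
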(event `self.ReceiveBeginPlay`
  (`KismetSystemLibrary.DelayUntilNextTick`)
  (bind _asbp_feather_hud (cast `/Game/Feather/Blueprints/Framework/BP_FeatherHUD` (`PlayerController.GetHUD` (`GameplayStatics.GetPlayerController` 0))))
  (set `self.Feather HUD` _asbp_feather_hud))

(event `self.Box.OnComponentBeginOverlap`
  (params (OverlappedComponent :type "PrimitiveComponent Object Reference") (OtherActor :type "Actor Object Reference") (OtherComp :type "PrimitiveComponent Object Reference") (OtherBodyIndex :type Integer) (bFromSweep :type Boolean) (SweepResult :type "HitResult Structure (by ref)"))
  (if (not (`self.DoOnce`))
    (cast `/Game/Feather/Blueprints/FeatherCharacter/BP_KiwiCharacter` OtherActor)
    (`/Game/Feather/Blueprints/Framework/BP_FeatherHUD.ShowLoreText` (`self.Feather HUD`) (`self.In Text`) (`self.Duration`))
    (set `self.DoOnce` (not (`self.IsRepeteable`)))))

(fn `UserConstructionScript`)