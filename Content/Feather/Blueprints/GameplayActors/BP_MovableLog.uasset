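; BP_MovableLog is a gameplay actor that moves its Cube mesh between a Start and an End component.
; On BeginPlay it sets the Movement timeline's play rate from MovementTime, then starts it immediately or after an optional StartDelay timer.
; Each timeline update lerps the Cube's world location between the two markers, without sweep or teleport.
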(event `self.ReceiveBeginPlay`
  (`TimelineComponent.SetPlayRate` (`self.Movement`) (/ 1.0 (`self.MovementTime`)))
  (if (> (`self.StartDelay`) 0.0)
    (`KismetSystemLibrary.K2_SetTimerDelegate` (delegate `Move`) (`self.StartDelay`))
    (else
      (`self.Move`))))

(event `Move`
  (bind (_direction _time) (`Timeline|Movement`)
    (:`Update`
      (`SceneComponent.K2_SetWorldLocation` (`self.Cube`) (`KismetMathLibrary.VLerp` (`SceneComponent.K2_GetComponentLocation` (`self.Start`)) (`SceneComponent.K2_GetComponentLocation` (`self.End`)) _time) false false))))

(fn `UserConstructionScript`)