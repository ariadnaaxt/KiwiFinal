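; BP_WinLevel is a trigger actor that ends a level when the player's kiwi character reaches its box.
; An overlap by either BP_KiwiCharacter or BP_SideScroller_KiwiCharacter waits briefly, then starts a comic using images retrieved from Configuration.
; The comic's finished callback async-loads the hardcoded MAP_Level3 and opens it by object reference.
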(event `self.Box.OnComponentBeginOverlap`
  (params (OverlappedComponent :type "PrimitiveComponent Object Reference") (OtherActor :type "Actor Object Reference") (OtherComp :type "PrimitiveComponent Object Reference") (OtherBodyIndex :type Integer) (bFromSweep :type Boolean) (SweepResult :type "HitResult Structure (by ref)"))
  (cast `/Game/Feather/Blueprints/FeatherCharacter/BP_KiwiCharacter` OtherActor
    (:`then`
      _)
    (:`CastFailed`
      (cast `/Game/Feather/Blueprints/FeatherCharacter/BP_SideScroller_KiwiCharacter` OtherActor)))
  (`KismetSystemLibrary.Delay` 1.0)
  (`/Game/Feather/Blueprints/Framework/BFL_Utils.StartComic` self (`/Game/Feather/Blueprints/DataAssets/PDA_Configuration.RetrieveComicImages` (`self.Configuration`) 2) (delegate `FinishedComic`)))

(event `FinishedComic`
  (`|LoadAsset` "/Game/Feather/Maps/MAP_Level3.MAP_Level3"
    (:`Completed`
      (`GameplayStatics.OpenLevelBySoftObjectPtr` (`self.Level`)))))

(fn `UserConstructionScript`)