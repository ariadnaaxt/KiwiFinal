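; BP_Tronco is a gameplay actor, apparently a tree trunk, that topples over on its own after a configurable initial delay.
; On BeginPlay it waits, then plays a timeline that rolls the Pivot component from its starting roll to 90 degrees with a sinusoidal ease-in.
; When the scripted fall finishes, it enables physics simulation on the Collider, handing motion over to the physics engine.
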(event `self.ReceiveBeginPlay`
  (`KismetSystemLibrary.Delay` (`self.InitialDelay`))
  (`self.FallingEvent`))

(event `FallingEvent`
  (bind _initial_rotation_roll (`KismetMathLibrary.BreakRotator` (`self.Initial Rotation`)))
  (bind (_initial_rotation_roll_2 _initial_rotation_pitch _initial_rotation_yaw) (`KismetMathLibrary.BreakRotator` (`self.Initial Rotation`)))
  (set `self.Initial Rotation` (`SceneComponent.RelativeRotation` (`self.Pivot`)))
  (bind (_direction _fallingcurve) (`Timeline|FallingTL` :!via `PlayFromStart`)
    (:`Update`
      (`SceneComponent.K2_SetRelativeRotation` (`self.Pivot`) (`KismetMathLibrary.MakeRotator` (`|EaseFunction` "SinusoidalIn" _fallingcurve _initial_rotation_roll 90.0) _initial_rotation_pitch _initial_rotation_yaw) false false))
    (:`Finished`
      (`self.EnablePhysics`))))

(event `EnablePhysics`
  (`PrimitiveComponent.SetSimulatePhysics` (`self.Collider`) true))

(fn `UserConstructionScript`)