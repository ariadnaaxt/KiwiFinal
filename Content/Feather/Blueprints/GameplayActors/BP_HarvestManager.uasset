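; Harvest manager Blueprint that shows the berry-picking quest objective ("Recoger bayas") on the Feather HUD.
; After a one-tick delay on BeginPlay, it caches the player's BP_FeatherHUD and binds to the harvest update and complete delegates.
; Updates rebuild the objective text from harvested and total counts; completion clears it after a short delay.
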(event `self.ReceiveBeginPlay`
  (`KismetSystemLibrary.DelayUntilNextTick`)
  (bind _asbp_feather_hud (cast `/Game/Feather/Blueprints/Framework/BP_FeatherHUD` (`PlayerController.GetHUD` (`GameplayStatics.GetPlayerController` 0))))
  (set `self.Feather HUD` _asbp_feather_hud)
  (add `self.OnHarvestedCompleteDelegate` (delegate `OnHarvestedCompleteDelegate_Event`))
  (add `self.OnHarvestedUpdateDelegate` (delegate `OnHarvestedUpdateDelegate_Event`)))

(event `OnHarvestedUpdateDelegate_Event`
  (`self.RefreshQuest`))

(event `OnHarvestedCompleteDelegate_Event`
  (`KismetSystemLibrary.Delay` 2.0)
  (`/Game/Feather/Blueprints/Framework/BP_FeatherHUD.SetObjectiveText` (`self.Feather HUD`) ""))

(event `RefreshQuest`
  (`/Game/Feather/Blueprints/Framework/BP_FeatherHUD.SetObjectiveText` (`self.Feather HUD`) (`KismetTextLibrary.Conv_StringToText` (`KismetStringLibrary.Concat_StrStr` "Recoger bayas " (`KismetStringLibrary.Conv_IntToString` (`self.HarvestedObjects`)) " / " (`KismetStringLibrary.Conv_IntToString` (`self.TotalObjects`))))))

(fn `UserConstructionScript`)